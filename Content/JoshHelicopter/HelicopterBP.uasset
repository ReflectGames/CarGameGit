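; Attack helicopter that repeatedly fires missiles, oriented toward the Sedan.
; A DoOnce-gated Tick spawns a HelicopterMissle at the right missile spawn, moves it along a randomly picked spline, then swaps it for a Missle after a delay.
; The random range starts at 1, so the first LeftSpline branch never runs.
; Construction attaches guns and propeller to mesh sockets; the alternating muzzle-flash and bullet gun logic is disconnected.
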(event `self.ReceiveTick`
  (params (DeltaSeconds :type "Float (single-precision)"))
  (`|ExecutionSequence`
    (:`then_1`
      (`/Engine/EditorBlueprintResources/StandardMacros.DoOnce` false :!label _label
        (:`Completed`
          (switch `int` (`KismetMathLibrary.RandomIntegerInRange` 1 6)
            (:`0`
              (bind _returnvalue (`|SpawnActorFromClass` "/Game/JoshHelicopter/HelicopterMissle.HelicopterMissle_C" (`KismetMathLibrary.Conv_VectorToTransform` (`SceneComponent.K2_GetComponentLocation` (`self.RightMissileSpawn`))) "Undefined" "OverrideRootScale"))
              (bind _returnvalue_2 (`iTween.ActorMoveToSplinePointFull` 0.0 "No Name" _returnvalue (`self.LeftSpline`) false true "none" false 0.0 "first" "seconds" 0.5 "linear" null 1.0 "rewind" 0 true "orientToTarget" "/Game/VehicleBP/Sedan/Sedan.Sedan" 1.0))
              (`KismetSystemLibrary.Delay` (`iTweenEvent.tickTypeValue` _returnvalue_2))
              (`|SpawnActorFromClass` "/Game/HomingFaggot/Missle.Missle_C" (`KismetMathLibrary.Conv_VectorToTransform` (`self.K2_GetActorLocation` _returnvalue)) "Undefined" "OverrideRootScale")
              (`self.K2_DestroyActor` _returnvalue)
              (goto _label :!via `Reset`))
            (:`1`
              (bind _returnvalue_3 (`|SpawnActorFromClass` "/Game/JoshHelicopter/HelicopterMissle.HelicopterMissle_C" (`KismetMathLibrary.Conv_VectorToTransform` (`SceneComponent.K2_GetComponentLocation` (`self.RightMissileSpawn`))) "Undefined" "OverrideRootScale"))
              (bind _returnvalue_4 (`iTween.ActorMoveToSplinePointFull` 0.0 "No Name" _returnvalue_3 (`self.RightSpline`) false true "none" false 0.0 "first" "seconds" 0.5 "linear" null 1.0 "rewind" 0 true "orientToTarget" "/Game/VehicleBP/Sedan/Sedan.Sedan" 2.0))
              (`KismetSystemLibrary.Delay` (`iTweenEvent.tickTypeValue` _returnvalue_4))
              (`|SpawnActorFromClass` "/Game/HomingFaggot/Missle.Missle_C" (`KismetMathLibrary.Conv_VectorToTransform` (`self.K2_GetActorLocation` _returnvalue_3)) "Undefined" "OverrideRootScale")
              (`self.K2_DestroyActor` _returnvalue_3)
              (goto _label :!via `Reset`))
            (:`2`
              (bind _returnvalue_5 (`|SpawnActorFromClass` "/Game/JoshHelicopter/HelicopterMissle.HelicopterMissle_C" (`KismetMathLibrary.Conv_VectorToTransform` (`SceneComponent.K2_GetComponentLocation` (`self.RightMissileSpawn`))) "Undefined" "OverrideRootScale"))
              (bind _returnvalue_6 (`iTween.ActorMoveToSplinePointFull` 0.0 "No Name" _returnvalue_5 (`self.LeftSpline2`) false true "none" false 0.0 "first" "seconds" 0.5 "linear" null 1.0 "rewind" 0 true "orientToTarget" "/Game/VehicleBP/Sedan/Sedan.Sedan" 1.0))
              (`KismetSystemLibrary.Delay` (`iTweenEvent.tickTypeValue` _returnvalue_6))
              (`|SpawnActorFromClass` "/Game/HomingFaggot/Missle.Missle_C" (`KismetMathLibrary.Conv_VectorToTransform` (`self.K2_GetActorLocation` _returnvalue_5)) "Undefined" "OverrideRootScale")
              (`self.K2_DestroyActor` _returnvalue_5)
              (goto _label :!via `Reset`))
            (:`3`
              (bind _returnvalue_7 (`|SpawnActorFromClass` "/Game/JoshHelicopter/HelicopterMissle.HelicopterMissle_C" (`KismetMathLibrary.Conv_VectorToTransform` (`SceneComponent.K2_GetComponentLocation` (`self.RightMissileSpawn`))) "Undefined" "OverrideRootScale"))
              (bind _returnvalue_8 (`iTween.ActorMoveToSplinePointFull` 0.0 "No Name" _returnvalue_7 (`self.RightSpline2`) false true "none" false 0.0 "first" "seconds" 0.5 "linear" null 1.0 "rewind" 0 true "orientToTarget" "/Game/VehicleBP/Sedan/Sedan.Sedan" 1.0))
              (`KismetSystemLibrary.Delay` (`iTweenEvent.tickTypeValue` _returnvalue_8))
              (`|SpawnActorFromClass` "/Game/HomingFaggot/Missle.Missle_C" (`KismetMathLibrary.Conv_VectorToTransform` (`self.K2_GetActorLocation` _returnvalue_7)) "Undefined" "OverrideRootScale")
              (`self.K2_DestroyActor` _returnvalue_7)
              (goto _label :!via `Reset`))
            (:`4`
              (bind _returnvalue_9 (`|SpawnActorFromClass` "/Game/JoshHelicopter/HelicopterMissle.HelicopterMissle_C" (`KismetMathLibrary.Conv_VectorToTransform` (`SceneComponent.K2_GetComponentLocation` (`self.RightMissileSpawn`))) "Undefined" "OverrideRootScale"))
              (bind _returnvalue_10 (`iTween.ActorMoveToSplinePointFull` 0.0 "No Name" _returnvalue_9 (`self.RightCenter`) false true "none" false 0.0 "first" "seconds" 0.5 "linear" null 1.0 "rewind" 0 true "orientToTarget" "/Game/VehicleBP/Sedan/Sedan.Sedan" 1.0))
              (`KismetSystemLibrary.Delay` (`iTweenEvent.tickTypeValue` _returnvalue_10))
              (`|SpawnActorFromClass` "/Game/HomingFaggot/Missle.Missle_C" (`KismetMathLibrary.Conv_VectorToTransform` (`self.K2_GetActorLocation` _returnvalue_9)) "Undefined" "OverrideRootScale")
              (`self.K2_DestroyActor` _returnvalue_9)
              (goto _label :!via `Reset`))
            (:`5`
              (bind _returnvalue_11 (`|SpawnActorFromClass` "/Game/JoshHelicopter/HelicopterMissle.HelicopterMissle_C" (`KismetMathLibrary.Conv_VectorToTransform` (`SceneComponent.K2_GetComponentLocation` (`self.RightMissileSpawn`))) "Undefined" "OverrideRootScale"))
              (bind _returnvalue_12 (`iTween.ActorMoveToSplinePointFull` 0.0 "No Name" _returnvalue_11 (`self.LeftCenter`) false true "none" false 0.0 "first" "seconds" 0.5 "linear" null 1.0 "rewind" 0 true "orientToTarget" "/Game/VehicleBP/Sedan/Sedan.Sedan" 1.0))
              (`KismetSystemLibrary.Delay` (`iTweenEvent.tickTypeValue` _returnvalue_12))
              (`|SpawnActorFromClass` "/Game/HomingFaggot/Missle.Missle_C" (`KismetMathLibrary.Conv_VectorToTransform` (`self.K2_GetActorLocation` _returnvalue_11)) "Undefined" "OverrideRootScale")
              (`self.K2_DestroyActor` _returnvalue_11)
              (goto _label :!via `Reset`))
            (:`6`
              (bind _returnvalue_13 (`|SpawnActorFromClass` "/Game/JoshHelicopter/HelicopterMissle.HelicopterMissle_C" (`KismetMathLibrary.Conv_VectorToTransform` (`SceneComponent.K2_GetComponentLocation` (`self.RightMissileSpawn`))) "Undefined" "OverrideRootScale"))
              (bind _returnvalue_14 (`iTween.ActorMoveToSplinePointFull` 0.0 "No Name" _returnvalue_13 (`self.Center`) false true "none" false 0.0 "first" "seconds" 0.5 "linear" null 1.0 "rewind" 0 true "orientToTarget" "/Game/VehicleBP/Sedan/Sedan.Sedan" 1.0))
              (`KismetSystemLibrary.Delay` (`iTweenEvent.tickTypeValue` _returnvalue_14))
              (`|SpawnActorFromClass` "/Game/HomingFaggot/Missle.Missle_C" (`KismetMathLibrary.Conv_VectorToTransform` (`self.K2_GetActorLocation` _returnvalue_13)) "Undefined" "OverrideRootScale")
              (`self.K2_DestroyActor` _returnvalue_13)
              (goto _label :!via `Reset`))))))))

(fn `UserConstructionScript`
  (`SceneComponent.K2_AttachToComponent` (`self.RGun`) (`self.SkeletalMesh`) "RSocket" "KeepWorld" "KeepWorld" "KeepWorld" true)
  (`SceneComponent.K2_AttachToComponent` (`self.LGun`) (`self.SkeletalMesh`) "LSocket" "KeepWorld" "KeepWorld" "KeepWorld" true)
  (`SceneComponent.K2_AttachToComponent` (`self.Propeller`) (`self.SkeletalMesh`) "PropellerSocket" "KeepWorld" "KeepWorld" "KeepWorld" true)
  (`SceneComponent.K2_AttachToComponent` (`self.RGun2`) (`self.SkeletalMesh`) "RSocket" "KeepWorld" "KeepWorld" "KeepWorld" true)
  (`SceneComponent.K2_AttachToComponent` (`self.LGun2`) (`self.SkeletalMesh`) "LSocket" "KeepWorld" "KeepWorld" "KeepWorld" true))