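; MultiplayerShellBP is a bullet shell actor that matches its casing mesh to the player's current weapon.
; On BeginPlay it reads weapon flags from NewGameInstance and equip state from the first Sedan found in the world.
; It toggles visibility of the 45Acp mesh for Glock or Mac10, or the Deagle mesh for Deagle.
; A Delay driven from Tick destroys the actor after twenty seconds.
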(event `self.ReceiveBeginPlay`
  (bind _asnew_game_instance (cast `/Game/MultiplayerStuff/NewGameInstance` (`GameplayStatics.GetGameInstance`)))
  (bind _outactors (`GameplayStatics.GetAllActorsOfClass` "/Game/VehicleBP/Sedan/Sedan.Sedan_C"))
  (bind _item (`KismetArrayLibrary.Array_Get` _outactors))
  (bind _returnvalue (or (`/Game/VehicleBP/Sedan/Sedan.SecondaryEquipped` _item) (`/Game/VehicleBP/Sedan/Sedan.HasNoPrimary` _item)))
  ;[1 1 1] Secondary Bullet Check
  (if (and (`/Game/MultiplayerStuff/NewGameInstance.Glock` _asnew_game_instance) _returnvalue)
    (`SceneComponent.ToggleVisibility` (`self.45_acp`) false)
    (elif (and (`/Game/MultiplayerStuff/NewGameInstance.Deagle` _asnew_game_instance) _returnvalue)
      (`SceneComponent.ToggleVisibility` (`self.Deagle`) false)
      (elif (and (`/Game/VehicleBP/Sedan/Sedan.PrimaryEquipped` _item) (`/Game/MultiplayerStuff/NewGameInstance.Mac10` _asnew_game_instance))
        (`SceneComponent.ToggleVisibility` (`self.45_acp`) false)))))

(event `self.ReceiveTick`
  (params (DeltaSeconds :type "Float (single-precision)"))
  (`KismetSystemLibrary.Delay` 20.0)
  (`self.K2_DestroyActor`))

(fn `UserConstructionScript`)