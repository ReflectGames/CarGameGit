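; MultiplayerShellBP is a shell casing actor for the multiplayer weapons.
; On BeginPlay it casts player pawn 0 to MultiplayerCharacter and toggles the 45Acp component's visibility if that character has the Glock or Mac10.
; Tick runs a Delay that destroys the actor about 20 seconds after it starts ticking.
; A disconnected branch for Deagle and primary-weapon visibility never runs.
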(event `self.ReceiveBeginPlay`
  (bind _asmultiplayer_character (cast `/Game/MultiplayerStuff/MultiplayerCharacter` (`GameplayStatics.GetPlayerPawn` 0)))
  ;[1 1 1] Secondary Bullet Check
  (if (or (`/Game/MultiplayerStuff/MultiplayerCharacter.HasGlock` _asmultiplayer_character) (`/Game/MultiplayerStuff/MultiplayerCharacter.HasMac10` _asmultiplayer_character))
    (`SceneComponent.ToggleVisibility` (`self.45_acp`) false)))

(event `self.ReceiveTick`
  (params (DeltaSeconds :type "Float (single-precision)"))
  (`KismetSystemLibrary.Delay` 20.0)
  (`self.K2_DestroyActor`))

(fn `UserConstructionScript`)