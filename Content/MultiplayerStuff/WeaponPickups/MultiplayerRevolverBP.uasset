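; Multiplayer revolver weapon Blueprint that handles hitscan shooting while ammo remains and player 0's MultiplayerCharacter holds the revolver.
; Fire decrements ammo, plays the shooting animation and line-traces for pawns from the first-person camera, ignoring the shooter, with debug drawing.
; It spawns a cosmetic bullet and a muzzle flash at the Muzzle socket, then calls ApplyDamage on the trace's hit actor without setting an amount.
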(event `Fire`
  (bind _revolver (`self.Revolver`))
  (if (> (`self.Ammo`) 0)
    (bind _asmultiplayer_character (cast `/Game/MultiplayerStuff/MultiplayerCharacter` (`GameplayStatics.GetPlayerPawn` 0)))
    (if (`/Game/MultiplayerStuff/MultiplayerCharacter.HasRevolver` _asmultiplayer_character)
      (`KismetSystemLibrary.PrintString` "Revolver Bang Bang")
      (set `self.Ammo` (- (`self.Ammo`) 1))
      (`SkeletalMeshComponent.PlayAnimation` (`self.Revolver`) "/Game/Test/Guns/Revolver/Revolver_Shooting.Revolver_Shooting" false)
      (bind _fpscamera (`/Game/MultiplayerStuff/MultiplayerCharacter.FpsCamera` _asmultiplayer_character))
      (bind _returnvalue (`SceneComponent.K2_GetComponentLocation` _fpscamera))
      (bind _outhit (`KismetSystemLibrary.LineTraceSingleForObjects` _returnvalue (+ _returnvalue (* (`SceneComponent.GetForwardVector` _fpscamera) 70000.0)) (`|MakeArray` "ObjectTypeQuery3" :!type "EObjectTypeQuery Enum") false (`|MakeArray` _asmultiplayer_character :!type "Actor Object Reference") "ForDuration"))
      ;[1 1 1] Spawn Asthetics
      (`|SpawnActorFromClass` "/Game/VehicleBP/Bullet.Bullet_C" (`KismetMathLibrary.MakeTransform` (`SceneComponent.K2_GetComponentLocation` (`self.Revolver`)) (`SceneComponent.K2_GetComponentRotation` (`/Game/MultiplayerStuff/MultiplayerCharacter.FpsCamera` _asmultiplayer_character))) "AlwaysSpawn" "OverrideRootScale")
      (`|SpawnActorFromClass` "/Game/MultiplayerStuff/MultiplayerRemakes/MultiplayerMuzzleFlash.MultiplayerMuzzleFlash_C" (`KismetMathLibrary.MakeTransform` (`SceneComponent.GetSocketLocation` _revolver "Muzzle") (`SceneComponent.GetSocketRotation` _revolver "Muzzle")) "AlwaysSpawn" "OverrideRootScale")
      (`GameplayStatics.ApplyDamage` (`.HitActor` (`GameplayStatics.BreakHitResult` _outhit)) 0.0 null self))))

(fn `UserConstructionScript`)