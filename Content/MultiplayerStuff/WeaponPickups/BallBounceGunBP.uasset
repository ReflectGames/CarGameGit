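; BallBounceGunBP is a multiplayer weapon Blueprint that fires bouncing ball projectiles.
; Its Fire event checks Ammo, casts player pawn 0 to MultiplayerCharacter and requires that character's HasBallBounce flag.
; It then decrements Ammo and spawns a scaled-down BouncingBalls actor at the FPS camera's location and rotation, owned by that character.
; The graph contains no pickup, replication or RPC logic.
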(event `Fire`
  (if (> (`self.Ammo`) 0)
    (bind _asmultiplayer_character (cast `/Game/MultiplayerStuff/MultiplayerCharacter` (`GameplayStatics.GetPlayerPawn` 0)))
    (if (`/Game/MultiplayerStuff/MultiplayerCharacter.HasBallBounce` _asmultiplayer_character)
      (set `self.Ammo` (- (`self.Ammo`) 1))
      (bind _fpscamera (`/Game/MultiplayerStuff/MultiplayerCharacter.FpsCamera` _asmultiplayer_character))
      (`|SpawnActorFromClass` "/Game/MultiplayerStuff/WeaponPickups/BallBounce/BouncingBalls.BouncingBalls_C" (`KismetMathLibrary.MakeTransform` (`SceneComponent.K2_GetComponentLocation` _fpscamera) (`SceneComponent.K2_GetComponentRotation` _fpscamera) (0.1 0.1 0.1)) "AlwaysSpawn" "OverrideRootScale" _asmultiplayer_character))))

(fn `UserConstructionScript`)