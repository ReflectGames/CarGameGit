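; Multiplayer shotgun weapon for the local player's character, handling firing and reloading.
; Fire line-traces a spread of pellets from the camera, doubles damage on Sitting or Arms component hits, and routes kills through FFAPlayerController's multicast or server death call.
; Shots spawn bullets, muzzle flash and an ejected shell behind a gate cooldown; an empty magazine switches to the Glock.
; Reload refills from reserve ammo, plays a montage and blocks firing until done.
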(event `Fire`
  (if (`self.CanFire`)
    (if (> (`self.Ammo`) 0)
      (bind _asmultiplayer_character (cast `/Game/MultiplayerStuff/MultiplayerCharacter` (`GameplayStatics.GetPlayerPawn` 0)))
      (if (`/Game/MultiplayerStuff/MultiplayerCharacter.Has Shotgun` _asmultiplayer_character)
        (`|ExecutionSequence`
          (:`then_0`
            (`/Engine/EditorBlueprintResources/StandardMacros.Gate` false :!label _label
              (:`Exit`
                (`|ExecutionSequence`
                  (:`then_0`
                    (for _ (range 9)
                      (bind _fpscamera (`/Game/MultiplayerStuff/MultiplayerCharacter.FpsCamera` _asmultiplayer_character))
                      (bind _returnvalue (`SceneComponent.K2_GetComponentLocation` _fpscamera))
                      (bind _returnvalue_2 (* (`SceneComponent.GetRightVector` _fpscamera) (`KismetMathLibrary.RandomFloatInRange` 0.0 50.0)))
                      (bind _returnvalue_3 (* (`SceneComponent.GetUpVector` _fpscamera) (`KismetMathLibrary.RandomFloatInRange` 0.0 50.0)))
                      (bind _outhit (`KismetSystemLibrary.LineTraceSingleForObjects` _returnvalue (+ (+ (+ _returnvalue (* (`SceneComponent.GetForwardVector` _fpscamera) 1500.0)) _returnvalue_2) _returnvalue_3) (`|MakeArray` "ObjectTypeQuery3" :!type "EObjectTypeQuery Enum") false (`|MakeArray` _asmultiplayer_character :!type "Actor Object Reference") "ForDuration"))
                      (`|ExecutionSequence`
                        (:`then_0`
                          (`|SpawnActorFromClass` "/Game/MultiplayerStuff/MultiplayerRemakes/MultiplayerShotgunBullet.MultiplayerShotgunBullet_C" (`KismetMathLibrary.MakeTransform` (+ (`SceneComponent.K2_GetComponentLocation` (`self.Shotgun`)) (+ _returnvalue_2 _returnvalue_3)) (`SceneComponent.K2_GetComponentRotation` (`/Game/MultiplayerStuff/MultiplayerCharacter.FpsCamera` _asmultiplayer_character)) (0.5 0.2 0.3)) "AlwaysSpawn" "OverrideRootScale"))
                        (:`then_1`
                          (bind (_bblockinghit _binitialoverlap _time _location _impactpoint _normal _impactnormal _physmat _hitactor _hitcomponent) (`GameplayStatics.BreakHitResult` _outhit))
                          (bind _asmultiplayer_character_2 (cast `/Game/MultiplayerStuff/MultiplayerCharacter` _hitactor))
                          (if (or (== (`/Game/MultiplayerStuff/MultiplayerCharacter.Sitting` _asmultiplayer_character_2) _hitcomponent) (== (`/Game/MultiplayerStuff/MultiplayerCharacter.Arms` _asmultiplayer_character_2) _hitcomponent))
                            (set `/Game/MultiplayerStuff/MultiplayerCharacter.Health` (- (`/Game/MultiplayerStuff/MultiplayerCharacter.Health` _asmultiplayer_character_2) (* (`self.Damage`) 2.0)) _asmultiplayer_character_2)
                            (else
                              (set `/Game/MultiplayerStuff/MultiplayerCharacter.Health` (- (`/Game/MultiplayerStuff/MultiplayerCharacter.Health` _asmultiplayer_character_2) (`self.Damage`)) _asmultiplayer_character_2)))
                          (set `/Game/MultiplayerStuff/MultiplayerCharacter.KillerRef` _asmultiplayer_character _asmultiplayer_character_2)
                          (if (not (> (`/Game/MultiplayerStuff/MultiplayerCharacter.Health` _asmultiplayer_character_2) 0.0))
                            (bind _asffaplayer_controller (cast `/Game/MultiplayerStuff/MultiplayerGameModes/FFAPlayerController` (`GameplayStatics.GetPlayerController` 0)))
                            (`/Engine/EditorBlueprintResources/ActorMacros.Switch Has Authority`
                              (:`Authority`
                                (`/Game/MultiplayerStuff/MultiplayerGameModes/FFAPlayerController.MulticastDie` _asffaplayer_controller _asmultiplayer_character_2))
                              (:`Remote`
                                (`/Game/MultiplayerStuff/MultiplayerGameModes/FFAPlayerController.ServerDie` _asffaplayer_controller _asmultiplayer_character_2))))))))
                  (:`then_1`
                    (bind _fpscamera_2 (`/Game/MultiplayerStuff/MultiplayerCharacter.FpsCamera` _asmultiplayer_character))
                    (`|SpawnActorFromClass` "/Game/MultiplayerStuff/MultiplayerRemakes/MultiplayerMuzzleFlash.MultiplayerMuzzleFlash_C" (`KismetMathLibrary.MakeTransform` (`SceneComponent.GetSocketLocation` (`self.Shotgun`) "Muzzle") (`SceneComponent.K2_GetComponentRotation` _fpscamera_2) (1.0 1.0 1.0)) "AlwaysSpawn" "OverrideRootScale")
                    (`GameplayStatics.PlaySoundAtLocation` "/Game/Gun-audio/shotgun.shotgun")
                    (bind _returnvalue_4 (`|SpawnActorFromClass` "/Game/Test/Shells/45acp/ShotgunShell.ShotgunShell_C" (`SceneComponent.GetSocketTransform` (`self.Shotgun`) "ShellEject" "RTS_World") "AlwaysSpawn" "OverrideRootScale"))
                    (bind _returnvalue_5 (`SceneComponent.K2_GetComponentRotation` _fpscamera_2))
                    (`PrimitiveComponent.AddImpulse` (`/Game/Test/Shells/45acp/ShotgunShell.ShotgunShell` _returnvalue_4) (+ (* (`KismetMathLibrary.GetRightVector` _returnvalue_5) (`KismetMathLibrary.RandomFloatInRange` -24.0 -5.0)) (* (`KismetMathLibrary.GetUpVector` _returnvalue_5) (`KismetMathLibrary.RandomFloatInRange` 6.0 10.0))) "None" false))
                  (:`then_2`
                    (`KismetSystemLibrary.Delay` 0.5)
                    (goto _label :!via `Open`))
                  (:`then_3`
                    (set `self.Ammo` (- (`self.Ammo`) 1)))))))
          (:`then_1`
            (goto _label :!via `Close`))))
      (else
        (bind _asmultiplayer_character_3 (cast `/Game/MultiplayerStuff/MultiplayerCharacter` (`GameplayStatics.GetPlayerPawn` 0)))
        (set `/Game/MultiplayerStuff/MultiplayerCharacter.Has Shotgun` false _asmultiplayer_character_3)
        (set `/Game/MultiplayerStuff/MultiplayerCharacter.HasGlock` true _asmultiplayer_character_3)))))

(event `Reload`
  (bind _asmultiplayer_character (cast `/Game/MultiplayerStuff/MultiplayerCharacter` (`GameplayStatics.GetPlayerPawn` 0)))
  (if (`/Game/MultiplayerStuff/MultiplayerCharacter.Has Shotgun` _asmultiplayer_character)
    (if (< (`self.Ammo`) 6)
      (if (> (`self.MaxAmmo`) 0)
        (`/Engine/EditorBlueprintResources/StandardMacros.DoOnce` false :!label _label_2
          (:`Completed`
            (`|ExecutionSequence`
              (:`then_0`
                (set `self.NeedAmmo` (- 6 (`self.Ammo`)))
                (if (<= (`self.MaxAmmo`) (`self.NeedAmmo`))
                  (set `self.Ammo` (+ (`self.Ammo`) (`self.MaxAmmo`)))
                  (set `self.MaxAmmo` 0)
                  (else
                    (set `self.MaxAmmo` (- (`self.MaxAmmo`) (`self.NeedAmmo`)))
                    (set `self.Ammo` 6))))
              (:`then_1`
                (set `self.CanFire` false)
                (`KismetSystemLibrary.Delay` 2.667)
                (set `self.CanFire` true)
                (goto _label_2 :!via `Reset`))
              (:`then_2`
                (`AnimInstance.Montage_Play` (`SkeletalMeshComponent.GetAnimInstance` (`/Game/MultiplayerStuff/MultiplayerCharacter.Arms` _asmultiplayer_character)) "/Game/AimTest/BasicArms/ReloadAnimMontage.ReloadAnimMontage" 1.0 "MontageLength" 0.0)))))))))

(fn `UserConstructionScript`)