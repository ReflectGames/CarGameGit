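; Multiplayer sticky bomb launcher weapon that decrements ammo on Fire and can preview a projectile arc, using player pawn 0.
; DrawProjectileTrajectory samples a gravity arc from the FPS camera's rotation, line tracing each segment until a hit.
; Alternate segments render as a dashed path of debug lines (set on BeginPlay) or beam particles.
; The right-mouse gate that would call the preview is disconnected, and Tick is empty.
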(event `Fire`
  (bind _asmultiplayer_character (cast `/Game/MultiplayerStuff/MultiplayerCharacter` (`GameplayStatics.GetPlayerPawn` 0)))
  (if (`/Game/MultiplayerStuff/MultiplayerCharacter.HasGrenadeLauncher` _asmultiplayer_character)
    (set `self.Ammo` (- (`self.Ammo`) 1))))

(event `self.ReceiveBeginPlay`
  ;[1 1 1] Trajectory
  (set `self.DrawingType` "NewEnumerator0"))

(event `self.ReceiveTick`
  (params (DeltaSeconds :type "Float (single-precision)"))
  ;[1 1 1] Trajectory
)

(event `DrawProjectileTrajectory`
  ;[1 1 1] Trajectory
  (bind _asmultiplayer_character (cast `/Game/MultiplayerStuff/MultiplayerCharacter` (`GameplayStatics.GetPlayerPawn` 0)))
  (`self.Clear Beams`)
  (bind _returnvalue (`SceneComponent.K2_GetComponentRotation` (`/Game/MultiplayerStuff/MultiplayerCharacter.FpsCamera` _asmultiplayer_character)))
  (bind _returnvalue_2 (+ (`SceneComponent.K2_GetComponentLocation` (`self.Sphere`)) (`KismetMathLibrary.GreaterGreater_VectorRotator` (`self.GunOffset`) _returnvalue)))
  (set `self. Start Location` _returnvalue_2)
  (set `self.Initial Velocity` (`KismetMathLibrary.TransformDirection` (`KismetMathLibrary.MakeTransform` _returnvalue_2 _returnvalue) (`self.Initial Local Velocity`)))
  (for _index (range (+ (`KismetMathLibrary.FFloor` (/ (`self.PathLifeTime`) (`self.TimeInterval`))) 1)) :!label _label
    (bind (_point_1 _point_2) (`self.Get Segment At Time` (`self. Start Location`) (`self.Initial Velocity`) (0.0 0.0 -980.0) (* _index (`self.TimeInterval`)) (* (+ _index 1) (`self.TimeInterval`))))
    (bind (_outhit _returnvalue_3) (`KismetSystemLibrary.LineTraceSingle` _point_1 _point_2 "TraceTypeQuery1" true))
    (`self.Visualize Segment` (`self.DrawingType`) _point_1 _point_2 _index)
    (if _returnvalue_3
      (`self.BreakDrawingLoop`))))

(event `BreakDrawingLoop`
  ;[1 1 1] Trajectory
  (goto _label :!via `Break`))

(fn `Add New Beam`
  (params (`Point 1` :type "Vector Structure") (`Point 2` :type "Vector Structure"))
  (bind _returnvalue (`AddComponent|NODE_AddParticleSystemComponent-0`))
  (`KismetArrayLibrary.Array_Add` (`self.BeamsArray`) _returnvalue)
  (`ParticleSystemComponent.SetBeamSourcePoint` _returnvalue 0 `Point 1` 0)
  (`ParticleSystemComponent.SetBeamSourcePoint` _returnvalue 0 `Point 2` 0))

(fn `Clear Beams`
  (bind _beamsarray (`self.BeamsArray`))
  (for _array_element _beamsarray
    (`ActorComponent.K2_DestroyComponent` _array_element))
  (`KismetArrayLibrary.Array_Clear` _beamsarray))

(fn `Get Segment At Time`
  (params (`Start Location` :type "Vector Structure") (`Initial Velocity` :type "Vector Structure") (Gravity :type "Vector Structure") (`Time 1` :type "Float (double-precision)") (`Time 2` :type "Float (double-precision)"))
  (returns (`Point 1` :type "Vector Structure") (`Point 2` :type "Vector Structure"))
  (return (+ `Start Location` (* `Initial Velocity` `Time 1`) (* Gravity (* `Time 1` `Time 1` 0.5))) (+ `Start Location` (* `Initial Velocity` `Time 2`) (* Gravity (* `Time 2` `Time 2` 0.5)))))

(fn `UserConstructionScript`)

(fn `Visualize Segment`
  (params (DrawingType :type "/Game/MultiplayerStuff/WeaponPickups/GrenadeLauncher/DrawingType Enum") (Point1 :type "Vector Structure") (Point2 :type "Vector Structure") (`Loop Index` :type Integer))
  (locals (Type :type "/Game/MultiplayerStuff/WeaponPickups/GrenadeLauncher/DrawingType Enum" :default "0") (P1 :type "Vector Structure") (P2 :type "Vector Structure"))
  (set `local.P1` Point1)
  (set `local.P2` Point2)
  (if (== (mod `Loop Index` 2) 0)
    (switch `/Game/MultiplayerStuff/WeaponPickups/GrenadeLauncher/DrawingType` DrawingType
      (:`NewEnumerator0`
        (`KismetSystemLibrary.DrawDebugLine` (`local.P1`) (`local.P2`) (struct :`R` 1.0 :`G` 0.32 :`B` 0.326982 :`A` 1.0) 0.0 2.0))
      (:`NewEnumerator1`
        (`self.Add New Beam` (`local.P1`) (`local.P2`))))))