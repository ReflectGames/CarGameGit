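; Multiplayer ball bounce gun that fires a chargeable projectile, growing bigger, slower and more damaging the longer it charges.
; Growing runs a gated delay loop that steps up a clamped Scale, while StopGrowing closes the gate and resets it.
; Fire checks ammo and the ball-bounce flag on player 0's character, spawns a FirstPersonProjectile along its camera rotation, then adjusts speed and damage by Scale.
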(event `Growing`
  (`|ExecutionSequence`
    (:`then_0`
      (goto _label :!via `Open`))
    (:`then_1`
      (`/Engine/EditorBlueprintResources/StandardMacros.Gate` true :!label _label
        (:`Exit`
          (set `self.Scale` (`KismetMathLibrary.ClampVectorSize` (+ (`self.Scale`) (0.1 0.1 0.1)) 0.0 3.0))
          (`KismetSystemLibrary.RetriggerableDelay` 0.2)
          (goto _label))))))

(event `Stop Growing`
  (set `self.Scale` (0.1 0.1 0.1))
  (goto _label :!via `Close`))

(event `Fire`
  (bind _returnvalue (+ (`self.Scale`) (0.1 0.1 0.1)))
  (bind _returnvalue_x (`KismetMathLibrary.BreakVector` (`KismetMathLibrary.ClampVectorSize` _returnvalue 0.0 5.0)))
  (bind _returnvalue_x_2 (`KismetMathLibrary.BreakVector` (`KismetMathLibrary.ClampVectorSize` _returnvalue 0.0 2.0)))
  (if (> (`self.Ammo`) 0)
    (bind _asmultiplayer_character (cast `/Game/MultiplayerStuff/MultiplayerCharacter` (`GameplayStatics.GetPlayerPawn` 0)))
    (if (`/Game/MultiplayerStuff/MultiplayerCharacter.HasBallBounce` _asmultiplayer_character)
      (set `self.Ammo` (- (`self.Ammo`) 1))
      (bind _returnvalue_2 (`|SpawnActorFromClass` "/Game/MultiplayerStuff/WeaponPickups/BallBounce/FirstPersonBP/Blueprints/FirstPersonProjectile.FirstPersonProjectile_C" (`KismetMathLibrary.MakeTransform` (`SceneComponent.K2_GetComponentLocation` (`self.Sphere`)) (`SceneComponent.K2_GetComponentRotation` (`/Game/MultiplayerStuff/MultiplayerCharacter.FpsCamera` _asmultiplayer_character)) (`self.Scale`)) "AlwaysSpawn" "OverrideRootScale" _asmultiplayer_character))
      (bind _projectile (`/Game/MultiplayerStuff/WeaponPickups/BallBounce/FirstPersonBP/Blueprints/FirstPersonProjectile.Projectile` _returnvalue_2))
      (set `ProjectileMovementComponent.InitialSpeed` (/ (`ProjectileMovementComponent.InitialSpeed` _projectile) _returnvalue_x_2) _projectile)
      (set `ProjectileMovementComponent.MaxSpeed` (/ (`ProjectileMovementComponent.MaxSpeed` _projectile) _returnvalue_x_2) _projectile)
      (set `/Game/MultiplayerStuff/WeaponPickups/BallBounce/FirstPersonBP/Blueprints/FirstPersonProjectile.Damage` (* _returnvalue_x (`/Game/MultiplayerStuff/WeaponPickups/BallBounce/FirstPersonBP/Blueprints/FirstPersonProjectile.Damage` _returnvalue_2)) _returnvalue_2))))

(fn `UserConstructionScript`)