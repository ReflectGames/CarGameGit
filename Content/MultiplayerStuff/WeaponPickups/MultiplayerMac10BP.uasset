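; Multiplayer Mac-10 weapon actor that handles automatic fire, ammo and reloading for player pawn 0.
; A gated retriggerable-delay loop line-traces from the FPS camera while spawning bullet, ejected shell and muzzle flash actors.
; Hits subtract the victim's Health directly, doubled on Sitting or Arms components, and record the killer.
; Reload refills from reserve with a montage and timed fire lockout; Tick restores ammo when the character flags ResetAmmo.
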(event `Fire`
  (bind _mac10 (`self.Mac10`))
  (bind _returnvalue (`SceneComponent.K2_GetComponentRotation` (`self.Mac10`)))
  (`|ExecutionSequence`
    (:`then_0`
      (goto _label :!via `Open`))
    (:`then_1`
      (`/Engine/EditorBlueprintResources/StandardMacros.Gate` true :!label _label
        (:`Exit`
          (if (> (`self.Ammo`) 0)
            (bind _asmultiplayer_character (cast `/Game/MultiplayerStuff/MultiplayerCharacter` (`GameplayStatics.GetPlayerPawn` 0)))
            (if (`/Game/MultiplayerStuff/MultiplayerCharacter.HasMac10` _asmultiplayer_character)
              (if (`self.CanFire`)
                (set `self.Ammo` (- (`self.Ammo`) 1))
                (`SkeletalMeshComponent.PlayAnimation` (`self.Mac10`) "/Game/Test/Guns/Mac-10/Mac-10_Untextured_Shooting_Anim.Mac-10_Untextured_Shooting_Anim" false)
                (bind _fpscamera (`/Game/MultiplayerStuff/MultiplayerCharacter.FpsCamera` _asmultiplayer_character))
                (bind _returnvalue_2 (`SceneComponent.K2_GetComponentLocation` _fpscamera))
                (bind _outhit (`KismetSystemLibrary.LineTraceSingleForObjects` _returnvalue_2 (+ _returnvalue_2 (* (`SceneComponent.GetForwardVector` _fpscamera) 70000.0)) (`|MakeArray` "ObjectTypeQuery3" :!type "EObjectTypeQuery Enum") false (`|MakeArray` _asmultiplayer_character :!type "Actor Object Reference") "ForDuration"))
                (`|ExecutionSequence`
                  (:`then_0`
                    ;[1 1 1] Spawn Asthetics
                    (`|SpawnActorFromClass` "/Game/VehicleBP/Bullet.Bullet_C" (`KismetMathLibrary.MakeTransform` (`SceneComponent.K2_GetComponentLocation` (`self.Mac10`)) (`SceneComponent.K2_GetComponentRotation` (`/Game/MultiplayerStuff/MultiplayerCharacter.FpsCamera` _asmultiplayer_character))) "AlwaysSpawn" "OverrideRootScale")
                    (bind _returnvalue_3 (`|SpawnActorFromClass` "/Game/MultiplayerStuff/MultiplayerRemakes/MultiplayerShellBP.MultiplayerShellBP_C" (`SceneComponent.GetSocketTransform` (`self.Mac10`) "BulletEject" "RTS_World") "Undefined" "OverrideRootScale"))
                    (`PrimitiveComponent.AddImpulse` (`/Game/MultiplayerStuff/MultiplayerRemakes/MultiplayerShellBP.45_acp` _returnvalue_3) (+ (* (`KismetMathLibrary.GetRightVector` _returnvalue) (`KismetMathLibrary.RandomFloatInRange` -7.0 -10.0)) (* (`KismetMathLibrary.GetUpVector` _returnvalue) (`KismetMathLibrary.RandomFloatInRange` 3.0 6.0))) "None" false)
                    (`PrimitiveComponent.AddImpulse` (`/Game/MultiplayerStuff/MultiplayerRemakes/MultiplayerShellBP.Deagle` _returnvalue_3) (+ (* (`KismetMathLibrary.GetRightVector` _returnvalue) (`KismetMathLibrary.RandomFloatInRange` -7.0 -10.0)) (* (`KismetMathLibrary.GetUpVector` _returnvalue) (`KismetMathLibrary.RandomFloatInRange` 3.0 6.0))) "None" false)
                    (`|SpawnActorFromClass` "/Game/MultiplayerStuff/MultiplayerRemakes/MultiplayerMuzzleFlash.MultiplayerMuzzleFlash_C" (`KismetMathLibrary.MakeTransform` (`SceneComponent.GetSocketLocation` _mac10 "Muzzle") (`SceneComponent.GetSocketRotation` _mac10 "Muzzle")) "AlwaysSpawn" "OverrideRootScale")
                    (bind (_bblockinghit _binitialoverlap _time _location _impactpoint _normal _impactnormal _physmat _hitactor _hitcomponent) (`GameplayStatics.BreakHitResult` _outhit))
                    (`GameplayStatics.ApplyDamage` _hitactor 0.0 null self)
                    (`KismetSystemLibrary.RetriggerableDelay` 0.05)
                    (goto _label))
                  (:`then_1`
                    (bind _asmultiplayer_character_2 (cast `/Game/MultiplayerStuff/MultiplayerCharacter` _hitactor))
                    (if (or (== (`/Game/MultiplayerStuff/MultiplayerCharacter.Sitting` _asmultiplayer_character_2) _hitcomponent) (== (`/Game/MultiplayerStuff/MultiplayerCharacter.Arms` _asmultiplayer_character_2) _hitcomponent))
                      (set `/Game/MultiplayerStuff/MultiplayerCharacter.Health` (- (`/Game/MultiplayerStuff/MultiplayerCharacter.Health` _asmultiplayer_character_2) (* (`self.Damage`) 2.0)) _asmultiplayer_character_2)
                      (else
                        (set `/Game/MultiplayerStuff/MultiplayerCharacter.Health` (- (`/Game/MultiplayerStuff/MultiplayerCharacter.Health` _asmultiplayer_character_2) (`self.Damage`)) _asmultiplayer_character_2)))
                    (set `/Game/MultiplayerStuff/MultiplayerCharacter.KillerRef` _asmultiplayer_character _asmultiplayer_character_2)))))))))))

(event `Stop Firing`
  (goto _label :!via `Close`))

(event `self.ReceiveBeginPlay`
  (set `self.CanFire` false)
  (set `self.CanFire` true))

(event `self.ReceiveTick`
  (params (DeltaSeconds :type "Float (single-precision)"))
  (`|ExecutionSequence`
    (:`then_0`
      (bind _asmultiplayer_character (cast `/Game/MultiplayerStuff/MultiplayerCharacter` (`GameplayStatics.GetPlayerPawn` 0)))
      (if (`/Game/MultiplayerStuff/MultiplayerCharacter.ResetAmmo` _asmultiplayer_character)
        (set `self.MaxAmmo` 90)
        (set `self.Ammo` 30)
        (set `/Game/MultiplayerStuff/MultiplayerCharacter.ResetAmmo` false _asmultiplayer_character)))))

(event `Reload`
  (bind _asmultiplayer_character (cast `/Game/MultiplayerStuff/MultiplayerCharacter` (`GameplayStatics.GetPlayerPawn` 0)))
  (if (`/Game/MultiplayerStuff/MultiplayerCharacter.HasMac10` _asmultiplayer_character)
    (if (< (`self.Ammo`) 30)
      (if (> (`self.MaxAmmo`) 0)
        (`/Engine/EditorBlueprintResources/StandardMacros.DoOnce` false :!label _label_2
          (:`Completed`
            (`|ExecutionSequence`
              (:`then_0`
                (set `self.NeedAmmo` (- 30 (`self.Ammo`)))
                (if (<= (`self.MaxAmmo`) (`self.NeedAmmo`))
                  (set `self.Ammo` (+ (`self.Ammo`) (`self.MaxAmmo`)))
                  (set `self.MaxAmmo` 0)
                  (else
                    (set `self.MaxAmmo` (- (`self.MaxAmmo`) (`self.NeedAmmo`)))
                    (set `self.Ammo` 30))))
              (:`then_1`
                (set `self.CanFire` false)
                (`KismetSystemLibrary.Delay` 2.667)
                (set `self.CanFire` true)
                (goto _label_2 :!via `Reset`))
              (:`then_2`
                (`AnimInstance.Montage_Play` (`SkeletalMeshComponent.GetAnimInstance` (`/Game/MultiplayerStuff/MultiplayerCharacter.Arms` _asmultiplayer_character)) "/Game/AimTest/BasicArms/ReloadAnimMontage.ReloadAnimMontage" 1.0 "MontageLength" 0.0)))))))))

(fn `UserConstructionScript`)