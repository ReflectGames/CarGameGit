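; Multiplayer Deagle weapon pickup that grants the gun to an overlapping MultiplayerCharacter.
; While its gate is open, Tick rotates the TriggerBox and plays a timeline whose Movement output offsets the actor locally.
; Any overlap closes the gate; a MultiplayerCharacter also gets HasDeagle set and the Mac10 and Glock flags cleared, then the pickup destroys itself.
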(event `self.ReceiveTick`
  (params (DeltaSeconds :type "Float (single-precision)"))
  (`/Engine/EditorBlueprintResources/StandardMacros.Gate` false :!label _label
    (:`Exit`
      (`SceneComponent.K2_AddRelativeRotation` (`self.TriggerBox`) (struct :`Yaw` 1.0) false false)
      (bind (_direction _movement) (`Timeline|Timeline_0`)
        (:`Update`
          (`self.K2_AddActorLocalOffset` _movement))))))

(event `self.TriggerBox.OnComponentBeginOverlap`
  (params (OverlappedComponent :type "PrimitiveComponent Object Reference") (OtherActor :type "Actor Object Reference") (OtherComp :type "PrimitiveComponent Object Reference") (OtherBodyIndex :type Integer) (bFromSweep :type Boolean) (SweepResult :type "HitResult Structure (by ref)"))
  (`|ExecutionSequence`
    (:`then_0`
      (goto _label :!via `Close`))
    (:`then_1`
      (bind _asmultiplayer_character (cast `/Game/MultiplayerStuff/MultiplayerCharacter` OtherActor))
      (set `/Game/MultiplayerStuff/MultiplayerCharacter.HasDeagle` true _asmultiplayer_character)
      (set `/Game/MultiplayerStuff/MultiplayerCharacter.HasMac10` false _asmultiplayer_character)
      (set `/Game/MultiplayerStuff/MultiplayerCharacter.HasGlock` false _asmultiplayer_character)
      (`self.K2_DestroyActor`))))

(fn `UserConstructionScript`)