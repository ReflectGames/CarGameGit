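; Multiplayer weapon pickup that gives an overlapping MultiplayerCharacter the ball bounce gun.
; Tick passes through a gate to spin the TriggerBox and play a timeline that offsets the actor for idle motion.
; Any overlap closes the gate; for a character, it switches the weapon boolean flags, flags an ammo reset and refills the child-actor gun's ammo.
; The pickup then destroys itself, with no authority check in this graph.
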(event `self.ReceiveTick`
  (params (DeltaSeconds :type "Float (single-precision)"))
  (`/Engine/EditorBlueprintResources/StandardMacros.Gate` false :!label _label
    (:`Exit`
      (`SceneComponent.K2_AddRelativeRotation` (`self.TriggerBox`) (struct :`Yaw` 1.0) false false)
      (bind (_direction _movement) (`Timeline|Timeline_0`)
        (:`Update`
          (`self.K2_AddActorLocalOffset` _movement))))))

(event `self.ReceiveActorBeginOverlap`
  (params (OtherActor :type "Actor Object Reference"))
  (`|ExecutionSequence`
    (:`then_0`
      (goto _label :!via `Close`))
    (:`then_1`
      (bind _asmultiplayer_character (cast `/Game/MultiplayerStuff/MultiplayerCharacter` OtherActor))
      (set `/Game/MultiplayerStuff/MultiplayerCharacter.ResetAmmo` true _asmultiplayer_character)
      (set `/Game/MultiplayerStuff/MultiplayerCharacter.HasBallBounce` true _asmultiplayer_character)
      (set `/Game/MultiplayerStuff/MultiplayerCharacter.HasDeagle` false _asmultiplayer_character)
      (set `/Game/MultiplayerStuff/MultiplayerCharacter.HasMac10` false _asmultiplayer_character)
      (set `/Game/MultiplayerStuff/MultiplayerCharacter.HasGrenadeLauncher` false _asmultiplayer_character)
      (set `/Game/MultiplayerStuff/MultiplayerCharacter.HasGlock` false _asmultiplayer_character)
      (set `/Game/MultiplayerStuff/MultiplayerCharacter.Has Shotgun` false _asmultiplayer_character)
      (set `/Game/MultiplayerStuff/MultiplayerCharacter.HasRevolver` false _asmultiplayer_character)
      (bind _asmultiplayer_ball_bounce_gun_bp (cast `/Game/MultiplayerStuff/WeaponPickups/MultiplayerBallBounceGunBP` (`ChildActorComponent.ChildActor` (`/Game/MultiplayerStuff/MultiplayerCharacter.BallBounceGun` _asmultiplayer_character))))
      (set `/Game/MultiplayerStuff/WeaponPickups/MultiplayerBallBounceGunBP.Ammo` 15 _asmultiplayer_ball_bounce_gun_bp)
      (`self.K2_DestroyActor`))))

(fn `UserConstructionScript`)