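; FlyingBotBP is a flying bot that turns to face the player vehicle class Sedan and animates its two thrusters.
; Every Tick it finds all Sedan actors and smoothly interpolates the Bot component's world rotation toward the first one with RInterpTo.
; It also randomizes each thruster's yaw and world scale every frame to produce a flickering exhaust effect.
; The bot never changes position.
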(event `self.ReceiveBeginPlay`)

(event `self.ReceiveTick`
  (params (DeltaSeconds :type "Float (single-precision)"))
  (bind _returnvalue (`KismetMathLibrary.RandomFloatInRange` 0.2 0.24))
  (bind _returnvalue_2 (`KismetMathLibrary.RandomFloatInRange` 0.2 0.24))
  (bind _bot (`self.Bot`))
  (bind _outactors (`GameplayStatics.GetAllActorsOfClass` "/Game/VehicleBP/Sedan/Sedan.Sedan_C"))
  (`SceneComponent.K2_SetWorldRotation` _bot (`KismetMathLibrary.RInterpTo` (`SceneComponent.K2_GetComponentRotation` _bot) (`KismetMathLibrary.FindLookAtRotation` (`SceneComponent.K2_GetComponentLocation` _bot) (`self.K2_GetActorLocation` (`KismetArrayLibrary.Array_Get` _outactors))) DeltaSeconds 1.0) false false)
  (`SceneComponent.K2_SetRelativeRotation` (`self.LThruster`) (`KismetMathLibrary.MakeRotator` 0.0 -90.0 (`KismetMathLibrary.RandomFloatInRange` 0.0 90.0)) false false)
  (`SceneComponent.K2_SetRelativeRotation` (`self.RThruster`) (`KismetMathLibrary.MakeRotator` 0.0 -90.0 (`KismetMathLibrary.RandomFloatInRange` 0.0 90.0)) false false)
  (`SceneComponent.SetWorldScale3D` (`self.LThruster`) (`KismetMathLibrary.MakeVector` (`KismetMathLibrary.RandomFloatInRange` 0.25 0.3) _returnvalue _returnvalue))
  (`SceneComponent.SetWorldScale3D` (`self.RThruster`) (`KismetMathLibrary.MakeVector` (`KismetMathLibrary.RandomFloatInRange` 0.25 0.3) _returnvalue_2 _returnvalue_2)))

(fn `UserConstructionScript`)