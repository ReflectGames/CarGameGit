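; Worm boss actor that performs a one-time burrow along a spline and leaves a hole behind.
; On the first Tick, a DoOnce sends the skeletal mesh to a spline point, using an arrow as orientation target, and plays the Burrow animation.
; After a short delay it spawns a Hole at a second arrow, which the construction script attaches to a mesh socket.
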(event `self.ReceiveTick`
  (params (DeltaSeconds :type "Float (single-precision)"))
  (`/Engine/EditorBlueprintResources/StandardMacros.DoOnce` false
    (:`Completed`
      (`iTween.ComponentMoveToSplinePointFull` 0.0 "No Name" (`self.SkeletalMesh`) (`self.Spline`) false true "none" false 0.0 "first" "seconds" 5.0 "linear" null 1.0 "once" 0 true "noOrientationChange" (`self.Arrow`))
      (`SkeletalMeshComponent.PlayAnimation` (`self.SkeletalMesh`) "/Game/WormBoss/Burrow.Burrow" false)
      (`KismetSystemLibrary.Delay` 1.35)
      (`|SpawnActorFromClass` "/Game/WormBoss/Hole.Hole_C" (`KismetMathLibrary.Conv_VectorToTransform` (`SceneComponent.K2_GetComponentLocation` (`self.Arrow1`))) "AlwaysSpawn" "OverrideRootScale"))))

(fn `UserConstructionScript`
  (`SceneComponent.K2_AttachToComponent` (`self.Arrow1`) (`self.SkeletalMesh`) "Socket" "KeepRelative" "KeepRelative" "KeepRelative" true))