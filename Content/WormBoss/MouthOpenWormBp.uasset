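; Open-mouth piece of the worm boss, with spinning, destructible teeth and trigger zones for the player's Sedan.
; Tick counter-rotates the Teeth and StaticMesh components until damage depletes TeethHealth, then destroys both once.
; Two overlap boxes respond only to the Sedan, one setting the LoseControl flag and the other clearing it.
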(event `self.ReceiveTick`
  (params (DeltaSeconds :type "Float (single-precision)"))
  (`|ExecutionSequence`
    (:`then_0`
      (if (<= (`self.TeethHealth`) 0.0)
        (`/Engine/EditorBlueprintResources/StandardMacros.DoOnce` false
          (:`Completed`
            (`ActorComponent.K2_DestroyComponent` (`self.Teeth`))
            (`ActorComponent.K2_DestroyComponent` (`self.StaticMesh`))))
        (else
          (`SceneComponent.K2_AddWorldRotation` (`self.Teeth`) (struct :`Roll` 0.2) false false)
          (`SceneComponent.K2_AddWorldRotation` (`self.StaticMesh`) (struct :`Roll` -0.4) false false))))))

(event `self.ReceiveAnyDamage`
  (params (Damage :type "Float (single-precision)") (DamageType :type "DamageType Object Reference") (InstigatedBy :type "Controller Object Reference") (DamageCauser :type "Actor Object Reference"))
  (bind _teethhealth (`self.TeethHealth`))
  (if (not (<= _teethhealth 0.0))
    (set `self.TeethHealth` (- _teethhealth Damage))))

(event `self.Box.OnComponentBeginOverlap`
  (params (OverlappedComponent :type "PrimitiveComponent Object Reference") (OtherActor :type "Actor Object Reference") (OtherComp :type "PrimitiveComponent Object Reference") (OtherBodyIndex :type Integer) (bFromSweep :type Boolean) (SweepResult :type "HitResult Structure (by ref)"))
  (cast `/Game/VehicleBP/Sedan/Sedan` OtherActor)
  (set `self.LoseControl` true))

(event `self.Box1.OnComponentBeginOverlap`
  (params (OverlappedComponent :type "PrimitiveComponent Object Reference") (OtherActor :type "Actor Object Reference") (OtherComp :type "PrimitiveComponent Object Reference") (OtherBodyIndex :type Integer) (bFromSweep :type Boolean) (SweepResult :type "HitResult Structure (by ref)"))
  (cast `/Game/VehicleBP/Sedan/Sedan` OtherActor)
  (set `self.LoseControl` false))

(fn `UserConstructionScript`)