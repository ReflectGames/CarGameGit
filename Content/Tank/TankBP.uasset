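; Enemy boss tank that drives toward the player, kills the Sedan on DieBox overlap and explodes into physics pieces at zero health.
; Tick runs two phases that StageCheck alternates by health thresholds, with damage accepted only in Phase1.
; Phase1 aims by line trace and fires TankBullet shells; Phase2 recenters the head and uses a reloading hitscan machine gun.
; Forward movement also scrolls tread material UVs.
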(event `self.ReceiveAnyDamage`
  (params (Damage :type "Float (single-precision)") (DamageType :type "DamageType Object Reference") (InstigatedBy :type "Controller Object Reference") (DamageCauser :type "Actor Object Reference"))
  (bind _tankhealth (`self.TankHealth`))
  (if (<= _tankhealth 0.0)
    _
    (elif (`self.Phase1`)
      (set `self.TankHealth` (- _tankhealth Damage)))))

(event `self.ReceiveBeginPlay`)

(event `self.ReceiveTick`
  (params (DeltaSeconds :type "Float (single-precision)"))
  (bind _machinegun (`self.MachineGun`))
  (bind _body (`self.Body`))
  (bind _forwardspeedstage2 (`self.ForwardSpeedStage2`))
  (bind _uvoffsetl (`self.UVOffsetL`))
  (bind _arrow (`self.Arrow`))
  (bind _forwardspeed (`self.ForwardSpeed`))
  (bind _returnvalue (`SceneComponent.K2_GetComponentLocation` _machinegun))
  (bind _returnvalue_2 (`SceneComponent.K2_GetComponentLocation` _arrow))
  (if (<= (`self.TankHealth`) 0.0)
    (`/Engine/EditorBlueprintResources/StandardMacros.DoOnce` false
      (:`Completed`
        (`GameplayStatics.SpawnEmitterAtLocation` "/Game/StarterContent/Particles/P_Explosion.P_Explosion" (`self.K2_GetActorLocation`) (struct))
        (`PrimitiveComponent.SetSimulatePhysics` (`self.LPlates`) true)
        (`PrimitiveComponent.SetSimulatePhysics` (`self.RPlates`) true)
        (`PrimitiveComponent.SetSimulatePhysics` (`self.LTreads`) true)
        (`PrimitiveComponent.SetSimulatePhysics` (`self.Tank_Cylinder`) true)
        (`PrimitiveComponent.SetSimulatePhysics` (`self.Head`) true)
        (`PrimitiveComponent.SetSimulatePhysics` _body true)
        (`PrimitiveComponent.SetSimulatePhysics` (`self.RTreads`) true)
        (`PrimitiveComponent.AddRadialImpulse` _body (`SceneComponent.K2_GetComponentLocation` _body) 5000.0 5000000.0 "RIF_Constant" false)
        (`PrimitiveComponent.SetCollisionEnabled` (`self.Box1`) "NoCollision")
        (`PrimitiveComponent.SetCollisionEnabled` (`self.Box2`) "NoCollision")
        (`PrimitiveComponent.SetCollisionEnabled` (`self.Die Box`) "NoCollision")
        (`PrimitiveComponent.SetCollisionEnabled` (`self.Box`) "NoCollision")))
    (else
      (`|ExecutionSequence`
        (:`then_0`
          (if (`self.Phase1`)
            ;[1 1 1] Turn Head
            (`|ExecutionSequence`
              (:`then_0`
                (bind _outactors (`GameplayStatics.GetAllActorsOfClass` "/Game/VehicleBP/Sedan/Sedan.Sedan_C"))
                (`SceneComponent.K2_SetWorldRotation` (`self.Arrow`) (`KismetMathLibrary.RInterpTo` (`SceneComponent.K2_GetComponentRotation` (`self.Arrow`)) (`KismetMathLibrary.MakeRotator` 0.0 (.pitch (`KismetMathLibrary.FindLookAtRotation` (`SceneComponent.K2_GetComponentLocation` (`self.Arrow`)) (`SceneComponent.K2_GetComponentLocation` (`/Game/VehicleBP/Sedan/Sedan.Homing Target Front` (`KismetArrayLibrary.Array_Get` _outactors))))) (.yaw (`KismetMathLibrary.FindLookAtRotation` (`SceneComponent.K2_GetComponentLocation` (`self.Arrow`)) (`SceneComponent.K2_GetComponentLocation` (`/Game/VehicleBP/Sedan/Sedan.Homing Target Front` (`KismetArrayLibrary.Array_Get` _outactors)))))) (`self.DeltaTime`) (`self.RotationSpeed`)) false false)
                (bind (_outhit _returnvalue_3) (`KismetSystemLibrary.LineTraceSingleForObjects` _returnvalue_2 (+ _returnvalue_2 (* (`SceneComponent.GetForwardVector` _arrow) 50000.0)) (`|MakeArray` "ObjectTypeQuery3" :!type "EObjectTypeQuery Enum") false (`|MakeArray` self :!type "Actor Object Reference") "ForOneFrame"))
                (if _returnvalue_3
                  (set `self.Locked On` true)
                  (`/Engine/EditorBlueprintResources/StandardMacros.DoOnce` false :!label _label
                    (:`Completed`
                      (`KismetSystemLibrary.RetriggerableDelay` 3.0)
                      (if (`self.Locked On`)
                        (`KismetSystemLibrary.PrintString` "Firing")
                        (set `self.RotationSpeed` 5.0)
                        (`KismetSystemLibrary.Delay` 2.0)
                        (`self.TankFire`)
                        (`KismetSystemLibrary.Delay` 3.0)
                        (set `self.Locked On` false)
                        (set `self.RotationSpeed` 0.0))))
                  (else
                    (set `self.Locked On` false)
                    (goto _label :!via `Reset`))))
              (:`then_1`
                (`|ExecutionSequence`
                  (:`then_0`
                    (set `self.DeltaTime` DeltaSeconds)
                    (`SceneComponent.K2_SetWorldRotation` (`self.Head`) (`KismetMathLibrary.RInterpTo` (`SceneComponent.K2_GetComponentRotation` (`self.Head`)) (`KismetMathLibrary.MakeRotator` 0.0 (.pitch (`KismetMathLibrary.FindLookAtRotation` (`SceneComponent.K2_GetComponentLocation` (`self.Head`)) (`self.K2_GetActorLocation` (`GameplayStatics.GetPlayerPawn` 0)))) (.yaw (`KismetMathLibrary.FindLookAtRotation` (`SceneComponent.K2_GetComponentLocation` (`self.Head`)) (`self.K2_GetActorLocation` (`GameplayStatics.GetPlayerPawn` 0))))) (`self.DeltaTime`) (`self.RotationSpeed`)) false false))
                  (:`then_2`
                    ;[1 1 1] Turn Body
                    (`self.K2_AddActorLocalRotation` (`KismetMathLibrary.MakeRotator` 0.0 0.0 (* (`KismetMathLibrary.MapRangeUnclamped` (.yaw (`KismetMathLibrary.NormalizedDeltaRotator` (`KismetMathLibrary.FindLookAtRotation` (`self.K2_GetActorLocation`) (`self.K2_GetActorLocation` (`GameplayStatics.GetPlayerPawn` 0))) (`self.K2_GetActorRotation`))) -90.0 90.0 -1.0 1.0) (`self.TurnSpeed`))))))))
            (elif (`self.Phase2`)
              (`|ExecutionSequence`
                (:`then_0`
                  (`SceneComponent.K2_SetWorldRotation` (`self.Head`) (`KismetMathLibrary.RInterpTo` (`SceneComponent.K2_GetComponentRotation` (`self.Head`)) (`KismetMathLibrary.MakeRotator` 0.0 0.0 (.yaw (`KismetMathLibrary.FindLookAtRotation` (`SceneComponent.K2_GetComponentLocation` (`self.Head`)) (`SceneComponent.K2_GetComponentLocation` (`self.ResetHead`))))) (`self.DeltaTime`) 1.0) false false))
                (:`then_1`
                  (`self.K2_AddActorLocalRotation` (`KismetMathLibrary.MakeRotator` 0.0 0.0 (* (`KismetMathLibrary.MapRangeUnclamped` (.yaw (`KismetMathLibrary.NormalizedDeltaRotator` (`KismetMathLibrary.FindLookAtRotation` (`self.K2_GetActorLocation`) (`self.K2_GetActorLocation` (`GameplayStatics.GetPlayerPawn` 0))) (`self.K2_GetActorRotation`))) -90.0 90.0 -1.0 1.0) 0.2))))
                (:`then_2`
                  (if (not (`self.OutOfAmmo`))
                    (`|ExecutionSequence`
                      (:`then_0`
                        (`KismetSystemLibrary.Delay` 0.2)
                        (bind (_outhit_2 _returnvalue_4) (`KismetSystemLibrary.LineTraceSingleForObjects` _returnvalue (+ _returnvalue (* (`SceneComponent.GetForwardVector` _machinegun) 50000.0)) (`|MakeArray` "ObjectTypeQuery3" :!type "EObjectTypeQuery Enum") false (`|MakeArray` self :!type "Actor Object Reference") "ForDuration"))
                        (if _returnvalue_4
                          (`GameplayStatics.ApplyDamage` (`.HitActor` (`GameplayStatics.BreakHitResult` _outhit_2)) (`self.MachineGunDmg`) null self)))
                      (:`then_1`
                        (`KismetSystemLibrary.Delay` 5.0)
                        (`KismetSystemLibrary.PrintString` "Reloading")
                        (set `self.OutOfAmmo` true)))))
                (:`then_3`
                  (bind _outactors_2 (`GameplayStatics.GetAllActorsOfClass` "/Game/VehicleBP/Sedan/Sedan.Sedan_C"))
                  (`SceneComponent.K2_SetWorldRotation` (`self.MachineGun`) (`KismetMathLibrary.RInterpTo` (`SceneComponent.K2_GetComponentRotation` (`self.MachineGun`)) (`KismetMathLibrary.MakeRotator` 0.0 (.pitch (`KismetMathLibrary.FindLookAtRotation` (`SceneComponent.K2_GetComponentLocation` (`self.MachineGun`)) (`SceneComponent.K2_GetComponentLocation` (`/Game/VehicleBP/Sedan/Sedan.Arms_Rig_Turn_Left` (`KismetArrayLibrary.Array_Get` _outactors_2))))) (.yaw (`KismetMathLibrary.FindLookAtRotation` (`SceneComponent.K2_GetComponentLocation` (`self.MachineGun`)) (`SceneComponent.K2_GetComponentLocation` (`/Game/VehicleBP/Sedan/Sedan.Arms_Rig_Turn_Left` (`KismetArrayLibrary.Array_Get` _outactors_2)))))) (`self.DeltaTime`) 2.0) true true))
                (:`then_4`
                  (if (`self.SpawnedGunner`)
                    (goto _label_2 :!via `Reset`)
                    (else
                      (`/Engine/EditorBlueprintResources/StandardMacros.DoOnce` false :!label _label_2
                        (:`Completed`
                          (bind _returnvalue_5 (`|SpawnActorFromClass` "/Game/Tank/TankGunner.TankGunner_C" (`KismetMathLibrary.Conv_VectorToTransform` (`SceneComponent.K2_GetComponentLocation` (`self.MachineGun`))) "AlwaysSpawn" "OverrideRootScale"))
                          (set `self.SpawnedGunner` true)
                          (`self.K2_AttachToComponent` _returnvalue_5 (`self.MachineGun`) "None" "KeepWorld" "KeepWorld" "KeepWorld" true))))))
                (:`then_5`
                  (if (`self.OutOfAmmo`)
                    (`KismetSystemLibrary.Delay` 5.0)
                    (`KismetSystemLibrary.PrintString` "Reloaded")
                    (set `self.OutOfAmmo` false)))))))
        (:`then_2`
          ;[1 1 1] Run Over
          (bind _outactors_3 (`GameplayStatics.GetAllActorsOfClass` "/Game/VehicleBP/Sedan/Sedan.Sedan_C"))
          (bind _item (`KismetArrayLibrary.Array_Get` _outactors_3))
          (if (`PrimitiveComponent.IsOverlappingComponent` (`WheeledVehicle.Mesh` _item) (`self.Die Box`))
            (set `/Game/VehicleBP/Sedan/Sedan.Health` 0.0 _item)
            (set `self.ForwardSpeed` 0.0)
            (set `self.TurnSpeed` 0.0)))
        (:`then_3`
          ;[1 1 1] UV Update
          (if (`self.Phase1`)
            (`self.K2_AddActorLocalOffset` (`KismetMathLibrary.MakeVector` _forwardspeed))
            (set `self.PositionOffset` _forwardspeed)
            (`self.UpdateTreadUVs` :!label _label_3)
            (`MeshComponent.SetScalarParameterValueOnMaterials` (`self.LTreads`) "TreadUVOffset" _uvoffsetl)
            (`MeshComponent.SetScalarParameterValueOnMaterials` (`self.RTreads`) "TreadUVOffset" _uvoffsetl)
            (elif (`self.Phase2`)
              (`self.K2_AddActorLocalOffset` (`KismetMathLibrary.MakeVector` _forwardspeedstage2))
              (set `self.PositionOffset` _forwardspeedstage2)
              (goto _label_3))))
        (:`then_4`
          (`self.StageCheck`))))))

(event `InputAxis|LookRight`
  (params (AxisValue :type "Float (single-precision)"))
  ;[1 1 1] Player Controls
  (`SceneComponent.K2_AddLocalRotation` (`self.Head`) (`KismetMathLibrary.MakeRotator` 0.0 0.0 (* AxisValue (`self.LookSpeedX`))) false false))

(event `InputAxis|LookUp`
  (params (AxisValue :type "Float (single-precision)"))
  ;[1 1 1] Player Controls
  (`SceneComponent.K2_AddLocalRotation` (`self.Head`) (`KismetMathLibrary.MakeRotator` 0.0 (* AxisValue (`self.LookSpeedY`))) false false))

(event `UpdateTreadUVs`
  (bind _output_get (set `self.OffsetL` (+ (`self.OffsetL`) (`self.PositionOffset`))))
  (set `self.UVOffsetL` (/ _output_get (/ (`self.TreadLength`) (`self.TreadUVTiles`)))))

(fn `CheckIfDead`
  (if (<= (`self.TankHealth`) 0.0)
    (`GameplayStatics.SpawnEmitterAtLocation` "/Game/StarterContent/Particles/P_Explosion.P_Explosion" (`self.K2_GetActorLocation`))
    (`PrimitiveComponent.SetSimulatePhysics` (`self.Tank_Cylinder`) true)
    (`PrimitiveComponent.SetSimulatePhysics` (`self.Head`) true)
    (`PrimitiveComponent.SetSimulatePhysics` (`self.Body`) true)
    (`PrimitiveComponent.SetSimulatePhysics` (`self.LTreads`) true)
    (`PrimitiveComponent.SetSimulatePhysics` (`self.LPlates`) true)
    (`PrimitiveComponent.SetSimulatePhysics` (`self.RPlates`) true)
    (`PrimitiveComponent.SetSimulatePhysics` (`self.RTreads`) true)
    (`ActorComponent.K2_DestroyComponent` (`self.Box1`))
    (`ActorComponent.K2_DestroyComponent` (`self.Box2`))
    (`ActorComponent.K2_DestroyComponent` (`self.Die Box`))
    (`ActorComponent.K2_DestroyComponent` (`self.Box`))))

(fn `StageCheck`
  (if (<= (`self.TankHealth`) 3750.0)
    (set `self.Phase1` false)
    (set `self.Phase2` true)
    (if (<= (`self.TankHealth`) 2500.0)
      (set `self.Phase2` false)
      (set `self.Phase1` true)
      (if (<= (`self.TankHealth`) 1250.0)
        (set `self.Phase1` false)
        (set `self.Phase2` true)))))

(fn `TankFire`
  (bind _arrow (`self.Arrow`))
  (`|SpawnActorFromClass` "/Game/Tank/TankBullet.TankBullet_C" (`KismetMathLibrary.MakeTransform` (+ (* (`SceneComponent.GetForwardVector` _arrow) 100.0) (`SceneComponent.K2_GetComponentLocation` _arrow)) (`SceneComponent.K2_GetComponentRotation` _arrow)) "Undefined" "OverrideRootScale"))

(fn `UserConstructionScript`)