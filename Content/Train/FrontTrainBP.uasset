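; Bandit train encounter actor that runs a front car and hooked carts along a spline once DidOverlap is set, using delayed per-car timelines.
; Tick randomly spawns BanditBP on cart spawn points up to a cap, then counts and destroys dead bandits to free slots.
; Reaching a kill threshold plays a hook animation and changes 1stBox collision.
; Damage depletes cart health, detaching the rear carts into physics.
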(event `self.ReceiveBeginPlay`
  (`|ExecutionSequence`
    (:`then_1`
      (`ActorComponent.Deactivate` (`self.1stBox`))
      (`ActorComponent.Deactivate` (`self.2ndBox`)))))

(event `self.ReceiveTick`
  (params (DeltaSeconds :type "Float (single-precision)"))
  (bind _t1setbandit (`self.T1SetBandit`))
  (bind _t1setbandit_2 (`self.T1SetBandit`))
  (bind _t1setbandit2 (`self.T1SetBandit2`))
  (bind _t1setbandit2_2 (`self.T1SetBandit2`))
  (bind _t1setbandit_3 (`self.T1SetBandit`))
  (bind _t1setbandit2_3 (`self.T1SetBandit2`))
  (bind _t3setbandit (`self.T3SetBandit`))
  (bind _t3setbandit_2 (`self.T3SetBandit`))
  (bind _t3setbandit_3 (`self.T3SetBandit`))
  (bind _t3setbandit2 (`self.T3SetBandit2`))
  (bind _t3setbandit2_2 (`self.T3SetBandit2`))
  (bind _t3setbandit2_3 (`self.T3SetBandit2`))
  (bind _t2setbandit2 (`self.T2SetBandit2`))
  (bind _t2setbandit (`self.T2SetBandit`))
  (bind _t2setbandit_2 (`self.T2SetBandit`))
  (bind _t2setbandit2_2 (`self.T2SetBandit2`))
  (bind _t2setbandit2_3 (`self.T2SetBandit2`))
  (bind _t2setbandit_3 (`self.T2SetBandit`))
  (bind _spline (`self.Spline`))
  (bind _spline_2 (`self.Spline`))
  (bind _spline_3 (`self.Spline`))
  (bind _spline_4 (`self.Spline`))
  (`|ExecutionSequence`
    (:`then_0`
      (if (`self.Did overlap?`)
        (`|ExecutionSequence`
          (:`then_0`
            (bind (_direction _animationalpha) (`Timeline|Timeline`)
              (:`Update`
                (bind _returnvalue (* (`SplineComponent.GetSplineLength` _spline_2) _animationalpha))
                (`SceneComponent.K2_SetWorldTransform` (`self.Front`) (`KismetMathLibrary.MakeTransform` (`SplineComponent.GetLocationAtDistanceAlongSpline` _spline_2 _returnvalue "World") (`SplineComponent.GetRotationAtDistanceAlongSpline` _spline_2 _returnvalue "World")) false false))))
          (:`then_1`
            (`KismetSystemLibrary.Delay` 0.563)
            (`KismetSystemLibrary.Delay` 0.563)
            (bind (_direction_2 _animationalpha_2) (`Timeline|Timeline_0`)
              (:`Update`
                (`SceneComponent.K2_SetWorldRotation` (`self.2ndCart`) (`SplineComponent.GetRotationAtDistanceAlongSpline` _spline_3 (* (`SplineComponent.GetSplineLength` _spline_3) _animationalpha_2) "World") false false))))
          (:`then_2`
            (`/Engine/EditorBlueprintResources/StandardMacros.DoOnce` false
              (:`Completed`
                (`KismetSystemLibrary.Delay` 1.016)
                (`KismetSystemLibrary.Delay` 1.016)
                (bind (_direction_3 _animationalpha_3) (`Timeline|Timeline_1`)
                  (:`Update`
                    (bind _returnvalue_2 (* (`SplineComponent.GetSplineLength` _spline_4) _animationalpha_3))
                    (`SceneComponent.K2_SetWorldTransform` (`self.3rdCart`) (`KismetMathLibrary.MakeTransform` (`SplineComponent.GetLocationAtDistanceAlongSpline` _spline_4 _returnvalue_2 "World") (`SplineComponent.GetRotationAtDistanceAlongSpline` _spline_4 _returnvalue_2 "World")) false false))))))
          (:`then_3`
            (`/Engine/EditorBlueprintResources/StandardMacros.DoOnce` false
              (:`Completed`
                (`KismetSystemLibrary.Delay` 1.38)
                (`KismetSystemLibrary.Delay` 1.38)
                (bind (_direction_4 _animationalpha_4) (`Timeline|Timeline_2` :!label _label)
                  (:`Update`
                    (bind _returnvalue_3 (* (`SplineComponent.GetSplineLength` _spline) _animationalpha_4))
                    (`SceneComponent.K2_SetWorldTransform` (`self.4thCart`) (`KismetMathLibrary.MakeTransform` (`SplineComponent.GetLocationAtDistanceAlongSpline` _spline _returnvalue_3 "World") (`SplineComponent.GetRotationAtDistanceAlongSpline` _spline _returnvalue_3 "World")) false false))))))
          (:`then_4`
            (if (== (`self.Killed`) 15.0)
              (`/Engine/EditorBlueprintResources/StandardMacros.DoOnce` false
                (:`Completed`
                  (`KismetSystemLibrary.Delay` 5.0)
                  (`SkeletalMeshComponent.PlayAnimation` (`self.3rdCart`) "/Game/Train/3rdCart/TrainCart3_Hook_Animation.TrainCart3_Hook_Animation" false)
                  (`|ExecutionSequence`
                    (:`then_0`
                      (goto _label :!via `Stop`))
                    (:`then_1`
                      (`KismetSystemLibrary.Delay` 0.0417)
                      (`PrimitiveComponent.SetCollisionObjectType` (`self.1stBox`) "ECC_Pawn")))))))
          (:`then_5`
            (`|ExecutionSequence`
              (:`then_0`
                (if (not (and (and (`self.T1Spawn1 Taken`) (`self.T1Spawn2 Taken`)) (and (and (`self.T2Spawn1 Taken`) (`self.T2Spawn2 Taken`)) (and (`self.T3Spawn1Taken`) (`self.T3Spawn2Taken`)))))
                  (`/Engine/EditorBlueprintResources/StandardMacros.DoOnce` false :!label _label_2
                    (:`Completed`
                      (`KismetSystemLibrary.Delay` 1.0)
                      (switch `int` (`KismetMathLibrary.RandomIntegerInRange` 0 2) :!label _label_3
                        (:`0`
                          (`|ExecutionSequence`
                            (:`then_0`
                              (if (`self.1stDead`)
                                _
                                (elif (< (`self.SpawnAmount`) 15)
                                  (switch `int` (`KismetMathLibrary.RandomIntegerInRange` 0 1)
                                    (:`0`
                                      (if (`self.T1Spawn1 Taken`)
                                        _
                                        (else
                                          (bind _returnvalue_4 (`|SpawnActorFromClass` "/Game/Train/Bandit/BanditDontDeleteThisOne/BanditBp.BanditBP_C" (`KismetMathLibrary.Conv_VectorToTransform` (`SceneComponent.K2_GetComponentLocation` (`self.T1 Spawn1`))) "Undefined" "OverrideRootScale"))
                                          (bind _output_get (set `self.T1SetBandit` _returnvalue_4))
                                          (`SceneComponent.K2_AttachToComponent` (`/Game/Train/Bandit/BanditDontDeleteThisOne/BanditBp.DefaultSceneRoot` _output_get) (`self.4thCart`) "None" "KeepWorld" "KeepWorld" "KeepWorld" true)
                                          (set `self.SpawnAmount` (+ (`self.SpawnAmount`) 1))
                                          (set `self.T1Spawn1 Taken` true)
                                          (goto _label_2 :!via `Reset`))))
                                    (:`1`
                                      _))
                                  (if (`self.T1Spawn2 Taken`)
                                    (goto _label_3)
                                    (else
                                      (bind _returnvalue_5 (`|SpawnActorFromClass` "/Game/Train/Bandit/BanditDontDeleteThisOne/BanditBp.BanditBP_C" (`KismetMathLibrary.Conv_VectorToTransform` (`SceneComponent.K2_GetComponentLocation` (`self.T1 Spawn2`))) "Undefined" "OverrideRootScale"))
                                      (bind _output_get_2 (set `self.T1SetBandit2` _returnvalue_5))
                                      (`SceneComponent.K2_AttachToComponent` (`/Game/Train/Bandit/BanditDontDeleteThisOne/BanditBp.DefaultSceneRoot` _output_get_2) (`self.4thCart`) "None" "KeepWorld" "KeepWorld" "KeepWorld" true)
                                      (set `self.SpawnAmount` (+ (`self.SpawnAmount`) 1))
                                      (set `self.T1Spawn2 Taken` true)
                                      (goto _label_2 :!via `Reset`))))))))
                        (:`1`
                          (`|ExecutionSequence`
                            (:`then_0`
                              (if (`self.2ndDead`)
                                _
                                (elif (< (`self.SpawnAmount`) 15)
                                  (switch `int` (`KismetMathLibrary.RandomIntegerInRange` 0 1)
                                    (:`0`
                                      (if (`self.T2Spawn1 Taken`)
                                        _
                                        (else
                                          (bind _returnvalue_6 (`|SpawnActorFromClass` "/Game/Train/Bandit/BanditDontDeleteThisOne/BanditBp.BanditBP_C" (`KismetMathLibrary.Conv_VectorToTransform` (`SceneComponent.K2_GetComponentLocation` (`self.T2 Spawn1`))) "Undefined" "OverrideRootScale"))
                                          (bind _output_get_3 (set `self.T2SetBandit` _returnvalue_6))
                                          (`SceneComponent.K2_AttachToComponent` (`/Game/Train/Bandit/BanditDontDeleteThisOne/BanditBp.DefaultSceneRoot` _output_get_3) (`self.3rdCart`) "None" "KeepWorld" "KeepWorld" "KeepWorld" true)
                                          (set `self.SpawnAmount` (+ (`self.SpawnAmount`) 1))
                                          (set `self.T2Spawn1 Taken` true)
                                          (goto _label_2 :!via `Reset`))))
                                    (:`1`
                                      _))
                                  (if (`self.T2Spawn2 Taken`)
                                    (goto _label_3)
                                    (else
                                      (bind _returnvalue_7 (`|SpawnActorFromClass` "/Game/Train/Bandit/BanditDontDeleteThisOne/BanditBp.BanditBP_C" (`KismetMathLibrary.Conv_VectorToTransform` (`SceneComponent.K2_GetComponentLocation` (`self.T2 Spawn 2`))) "Undefined" "OverrideRootScale"))
                                      (bind _output_get_4 (set `self.T2SetBandit2` _returnvalue_7))
                                      (`SceneComponent.K2_AttachToComponent` (`/Game/Train/Bandit/BanditDontDeleteThisOne/BanditBp.DefaultSceneRoot` _output_get_4) (`self.3rdCart`) "None" "KeepWorld" "KeepWorld" "KeepWorld" true)
                                      (set `self.SpawnAmount` (+ (`self.SpawnAmount`) 1))
                                      (set `self.T2Spawn2 Taken` true)
                                      (goto _label_2 :!via `Reset`))))))))
                        (:`2`
                          (`|ExecutionSequence`
                            (:`then_0`
                              (if (`self.3rdDead`)
                                _
                                (elif (< (`self.SpawnAmount`) 15)
                                  (switch `int` (`KismetMathLibrary.RandomIntegerInRange` 0 1)
                                    (:`0`
                                      (if (`self.T3Spawn1Taken`)
                                        _
                                        (else
                                          (bind _returnvalue_8 (`|SpawnActorFromClass` "/Game/Train/Bandit/BanditDontDeleteThisOne/BanditBp.BanditBP_C" (`KismetMathLibrary.Conv_VectorToTransform` (`SceneComponent.K2_GetComponentLocation` (`self.T3 Spawn1`))) "Undefined" "OverrideRootScale"))
                                          (bind _output_get_5 (set `self.T3SetBandit` _returnvalue_8))
                                          (`SceneComponent.K2_AttachToComponent` (`/Game/Train/Bandit/BanditDontDeleteThisOne/BanditBp.DefaultSceneRoot` _output_get_5) (`self.2ndCart`) "None" "KeepWorld" "KeepWorld" "KeepWorld" true)
                                          (set `self.SpawnAmount` (+ (`self.SpawnAmount`) 1))
                                          (set `self.T3Spawn1Taken` true)
                                          (goto _label_2 :!via `Reset`))))
                                    (:`1`
                                      _))
                                  (if (`self.T3Spawn2Taken`)
                                    (goto _label_3)
                                    (else
                                      (bind _returnvalue_9 (`|SpawnActorFromClass` "/Game/Train/Bandit/BanditDontDeleteThisOne/BanditBp.BanditBP_C" (`KismetMathLibrary.Conv_VectorToTransform` (`SceneComponent.K2_GetComponentLocation` (`self.T3 Spawn2`))) "Undefined" "OverrideRootScale"))
                                      (bind _output_get_6 (set `self.T3SetBandit2` _returnvalue_9))
                                      (`SceneComponent.K2_AttachToComponent` (`/Game/Train/Bandit/BanditDontDeleteThisOne/BanditBp.DefaultSceneRoot` _output_get_6) (`self.2ndCart`) "None" "KeepWorld" "KeepWorld" "KeepWorld" true)
                                      (set `self.SpawnAmount` (+ (`self.SpawnAmount`) 1))
                                      (set `self.T3Spawn2Taken` true)
                                      (goto _label_2 :!via `Reset`)))))))))))))
              (:`then_1`
                (`|ExecutionSequence`
                  (:`then_0`
                    (`|ExecutionSequence`
                      (:`then_0`
                        (`/Engine/EditorBlueprintResources/StandardMacros.IsValid` _t1setbandit_3
                          (:`Is Valid`
                            (if (<= (`/Game/Train/Bandit/BanditDontDeleteThisOne/BanditBp.BanditHealth` _t1setbandit_3) 0.0)
                              (`/Engine/EditorBlueprintResources/StandardMacros.IsValid` (`self.T1SetBandit`)
                                (:`Is Valid`
                                  (set `self.Killed` (+ (`self.Killed`) 1.0))
                                  (set `self.T1Spawn1 Taken` false)))))))
                      (:`then_1`
                        (`/Engine/EditorBlueprintResources/StandardMacros.IsValid` _t1setbandit2_3
                          (:`Is Valid`
                            (if (<= (`/Game/Train/Bandit/BanditDontDeleteThisOne/BanditBp.BanditHealth` _t1setbandit2_3) 0.0)
                              (`/Engine/EditorBlueprintResources/StandardMacros.IsValid` (`self.T1SetBandit2`)
                                (:`Is Valid`
                                  (set `self.Killed` (+ (`self.Killed`) 1.0))
                                  (set `self.T1Spawn2 Taken` false)))))))
                      (:`then_2`
                        (`/Engine/EditorBlueprintResources/StandardMacros.IsValid` _t1setbandit
                          (:`Is Valid`
                            (if (<= (`/Game/Train/Bandit/BanditDontDeleteThisOne/BanditBp.BanditHealth` _t1setbandit) 0.0)
                              (`/Engine/EditorBlueprintResources/StandardMacros.IsValid` _t1setbandit_2
                                (:`Is Valid`
                                  (`self.K2_DestroyActor` _t1setbandit_2)))))))
                      (:`then_4`
                        (`/Engine/EditorBlueprintResources/StandardMacros.IsValid` _t1setbandit2
                          (:`Is Valid`
                            (if (<= (`/Game/Train/Bandit/BanditDontDeleteThisOne/BanditBp.BanditHealth` _t1setbandit2) 0.0)
                              (`/Engine/EditorBlueprintResources/StandardMacros.IsValid` _t1setbandit2_2
                                (:`Is Valid`
                                  (`self.K2_DestroyActor` _t1setbandit2_2)))))))))
                  (:`then_1`
                    (`|ExecutionSequence`
                      (:`then_0`
                        (`/Engine/EditorBlueprintResources/StandardMacros.IsValid` _t2setbandit_3
                          (:`Is Valid`
                            (if (<= (`/Game/Train/Bandit/BanditDontDeleteThisOne/BanditBp.BanditHealth` _t2setbandit_3) 0.0)
                              (`/Engine/EditorBlueprintResources/StandardMacros.IsValid` (`self.T2SetBandit`)
                                (:`Is Valid`
                                  (set `self.Killed` (+ (`self.Killed`) 1.0))
                                  (set `self.T2Spawn1 Taken` false)))))))
                      (:`then_1`
                        (`/Engine/EditorBlueprintResources/StandardMacros.IsValid` _t2setbandit2
                          (:`Is Valid`
                            (if (<= (`/Game/Train/Bandit/BanditDontDeleteThisOne/BanditBp.BanditHealth` _t2setbandit2) 0.0)
                              (`/Engine/EditorBlueprintResources/StandardMacros.IsValid` (`self.T2SetBandit2`)
                                (:`Is Valid`
                                  (set `self.Killed` (+ (`self.Killed`) 1.0))
                                  (set `self.T2Spawn2 Taken` false)))))))
                      (:`then_2`
                        (`/Engine/EditorBlueprintResources/StandardMacros.IsValid` _t2setbandit_2
                          (:`Is Valid`
                            (if (<= (`/Game/Train/Bandit/BanditDontDeleteThisOne/BanditBp.BanditHealth` _t2setbandit_2) 0.0)
                              (`/Engine/EditorBlueprintResources/StandardMacros.IsValid` _t2setbandit
                                (:`Is Valid`
                                  (`self.K2_DestroyActor` _t2setbandit)))))))
                      (:`then_4`
                        (`/Engine/EditorBlueprintResources/StandardMacros.IsValid` _t2setbandit2_3
                          (:`Is Valid`
                            (if (<= (`/Game/Train/Bandit/BanditDontDeleteThisOne/BanditBp.BanditHealth` _t2setbandit2_3) 0.0)
                              (`/Engine/EditorBlueprintResources/StandardMacros.IsValid` _t2setbandit2_2
                                (:`Is Valid`
                                  (`self.K2_DestroyActor` _t2setbandit2_2)))))))))
                  (:`then_2`
                    (`|ExecutionSequence`
                      (:`then_0`
                        (`/Engine/EditorBlueprintResources/StandardMacros.IsValid` _t3setbandit_3
                          (:`Is Valid`
                            (if (<= (`/Game/Train/Bandit/BanditDontDeleteThisOne/BanditBp.BanditHealth` _t3setbandit_3) 0.0)
                              (`/Engine/EditorBlueprintResources/StandardMacros.IsValid` (`self.T3SetBandit`)
                                (:`Is Valid`
                                  (set `self.Killed` (+ (`self.Killed`) 1.0))
                                  (set `self.T3Spawn1Taken` false)))))))
                      (:`then_1`
                        (`/Engine/EditorBlueprintResources/StandardMacros.IsValid` _t3setbandit2_3
                          (:`Is Valid`
                            (if (<= (`/Game/Train/Bandit/BanditDontDeleteThisOne/BanditBp.BanditHealth` _t3setbandit2_3) 0.0)
                              (`/Engine/EditorBlueprintResources/StandardMacros.IsValid` (`self.T3SetBandit2`)
                                (:`Is Valid`
                                  (set `self.Killed` (+ (`self.Killed`) 1.0))
                                  (set `self.T3Spawn2Taken` false)))))))
                      (:`then_2`
                        (`/Engine/EditorBlueprintResources/StandardMacros.IsValid` _t3setbandit
                          (:`Is Valid`
                            (if (<= (`/Game/Train/Bandit/BanditDontDeleteThisOne/BanditBp.BanditHealth` _t3setbandit) 0.0)
                              (`/Engine/EditorBlueprintResources/StandardMacros.IsValid` _t3setbandit_2
                                (:`Is Valid`
                                  (`self.K2_DestroyActor` _t3setbandit_2)))))))
                      (:`then_4`
                        (`/Engine/EditorBlueprintResources/StandardMacros.IsValid` _t3setbandit2
                          (:`Is Valid`
                            (if (<= (`/Game/Train/Bandit/BanditDontDeleteThisOne/BanditBp.BanditHealth` _t3setbandit2) 0.0)
                              (`/Engine/EditorBlueprintResources/StandardMacros.IsValid` _t3setbandit2_2
                                (:`Is Valid`
                                  (`self.K2_DestroyActor` _t3setbandit2_2))))))))))))))))
    (:`then_1`
      (if (== (`self.Killed`) 30.0)
        _))))

(event `self.ReceiveAnyDamage`
  (params (Damage :type "Float (single-precision)") (DamageType :type "DamageType Object Reference") (InstigatedBy :type "Controller Object Reference") (DamageCauser :type "Actor Object Reference"))
  (bind _3rdcart (`self.3rdCart`))
  (bind _4thcart (`self.4thCart`))
  (if (`self.1stDead`)
    (if (`self.2ndDead`)
      _
      (elif (> (`self.2ndHealth`) 0.0)
        (set `self.2ndHealth` (- (`self.2ndHealth`) Damage))
        (else
          (`SceneComponent.K2_DetachFromComponent` (`self.3rdCart`) "KeepWorld" "KeepWorld" "KeepWorld" true)
          (`PrimitiveComponent.SetCollisionEnabled` _3rdcart "QueryAndPhysics")
          (`PrimitiveComponent.SetSimulatePhysics` _3rdcart true))))
    (elif (> (`self.1stHealth`) 0.0)
      (set `self.1stHealth` (- (`self.1stHealth`) Damage))
      (else
        (`SceneComponent.K2_DetachFromComponent` (`self.4thCart`) "KeepWorld" "KeepWorld" "KeepWorld" true)
        (`PrimitiveComponent.SetCollisionEnabled` _4thcart "QueryAndPhysics")
        (`PrimitiveComponent.SetSimulatePhysics` _4thcart true)
        (`PrimitiveComponent.SetCollisionEnabled` (`self.1stBox`) "NoCollision")
        (set `self.1stCanSpawn` false)
        (set `self.1stDead` true)))))

(fn `UserConstructionScript`
  (`SceneComponent.K2_AttachToComponent` (`self.PhysicsConstraint`) (`self.Front`) "Hook" "KeepWorld" "KeepWorld" "KeepWorld" true)
  (`SceneComponent.K2_AttachToComponent` (`self.2ndCart`) (`self.Front`) "Hook" "KeepRelative" "KeepWorld" "KeepWorld" true)
  (`SceneComponent.K2_AttachToComponent` (`self.3rdCart`) (`self.2ndCart`) "Hook" "KeepRelative" "KeepWorld" "KeepWorld" true)
  (`SceneComponent.K2_AttachToComponent` (`self.4thCart`) (`self.3rdCart`) "Hook" "KeepRelative" "KeepWorld" "KeepWorld" false))