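; BanditBp is an enemy train bandit that shoots at the Sedan and loses health when damaged.
; It plays a climb animation on spawn, then enables firing.
; Tick uses a Delay to pace debug-drawn, randomly spread line traces from the right gun, damaging hit pawns.
; Each tick also snaps the gun toward the first Sedan's arms rig and copies that yaw to the bandit mesh.
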(event `self.ReceiveAnyDamage`
  (params (Damage :type "Float (single-precision)") (DamageType :type "DamageType Object Reference") (InstigatedBy :type "Controller Object Reference") (DamageCauser :type "Actor Object Reference"))
  (bind _bandithealth (`self.BanditHealth`))
  (if (> _bandithealth 0.0)
    (set `self.BanditHealth` (- _bandithealth Damage))
    (else
      (`self.K2_DestroyActor`))))

(event `self.ReceiveBeginPlay`
  (`SkeletalMeshComponent.PlayAnimation` (`self.Bandit`) "/Game/Train/Bandit/BanditDontDeleteThisOne/Bandit_Climb_Anim.Bandit_Climb_Anim" false)
  (`KismetSystemLibrary.Delay` 1.667)
  (set `self.CanFire` true)
  (`SkeletalMeshComponent.PlayAnimation` (`self.Bandit`) "/Game/Train/Bandit/BanditDontDeleteThisOne/Bandit_Idle_Anim.Bandit_Idle_Anim" false))

(event `self.ReceiveTick`
  (params (DeltaSeconds :type "Float (single-precision)"))
  (bind _right_gun (`self.Right Gun`))
  (bind _right_gun_2 (`self.Right Gun`))
  (bind _returnvalue (`SceneComponent.K2_GetComponentLocation` _right_gun_2))
  (bind (_returnvalue_roll _returnvalue_pitch _returnvalue_yaw) (`KismetMathLibrary.BreakRotator` (`SceneComponent.K2_GetComponentRotation` (`self.Right Gun`))))
  (set `self.DeltaTime` DeltaSeconds)
  (if (`self.CanFire`)
    (`|ExecutionSequence`
      (:`then_1`
        (`KismetSystemLibrary.Delay` 1.0)
        (bind _outhit (`KismetSystemLibrary.LineTraceSingleForObjects` :`Start` _returnvalue :`End` (+ (+ (+ _returnvalue (* (`SceneComponent.GetForwardVector` _right_gun_2) 9000.0)) (* (`SceneComponent.GetRightVector` _right_gun_2) (`KismetMathLibrary.RandomFloatInRange` 0.0 550.0))) (* (`SceneComponent.GetUpVector` _right_gun_2) (`KismetMathLibrary.RandomFloatInRange` -100.0 100.0))) :`ObjectTypes` (`|MakeArray` "ObjectTypeQuery3" :!type "EObjectTypeQuery Enum") :`DrawDebugType` "ForDuration"))
        (`GameplayStatics.ApplyDamage` (`.HitActor` (`GameplayStatics.BreakHitResult` _outhit)) (`self.GunDamage`) null self))
      (:`then_2`
        (bind _outactors (`GameplayStatics.GetAllActorsOfClass` "/Game/VehicleBP/Sedan/Sedan.Sedan_C"))
        (`SceneComponent.K2_SetWorldRotation` _right_gun (`KismetMathLibrary.RInterpTo` (`SceneComponent.K2_GetComponentRotation` _right_gun) (`KismetMathLibrary.MakeRotator` (.roll (`KismetMathLibrary.FindLookAtRotation` (`SceneComponent.K2_GetComponentLocation` (`self.Right Gun`)) (`SceneComponent.K2_GetComponentLocation` (`/Game/VehicleBP/Sedan/Sedan.Arms_Rig_Turn_Left` (`KismetArrayLibrary.Array_Get` _outactors))))) (.pitch (`KismetMathLibrary.FindLookAtRotation` (`SceneComponent.K2_GetComponentLocation` (`self.Right Gun`)) (`SceneComponent.K2_GetComponentLocation` (`/Game/VehicleBP/Sedan/Sedan.Arms_Rig_Turn_Left` (`KismetArrayLibrary.Array_Get` _outactors))))) (.yaw (`KismetMathLibrary.FindLookAtRotation` (`SceneComponent.K2_GetComponentLocation` (`self.Right Gun`)) (`SceneComponent.K2_GetComponentLocation` (`/Game/VehicleBP/Sedan/Sedan.Arms_Rig_Turn_Left` (`KismetArrayLibrary.Array_Get` _outactors)))))) (`self.DeltaTime`) 0.0) true false)
        (`SceneComponent.K2_SetWorldRotation` (`self.Bandit`) (`KismetMathLibrary.MakeRotator` 0.0 0.0 _returnvalue_yaw) true false)))))

(fn `UserConstructionScript`)