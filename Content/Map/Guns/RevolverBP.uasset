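; RevolverBP is a revolver gun actor whose Firing function launches a shot.
; It spawns a Bullet at the actor location plus WeaponOffset rotated by the skeletal mesh's world rotation, facing that same rotation.
; It also runs a long, debug-drawn Camera-channel line trace forward from the Arrow component, but the hit result is unused.
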(fn `Firing`
  (bind _arrow (`self.Arrow`))
  (bind _returnvalue (`SceneComponent.K2_GetComponentRotation` (`self.SkeletalMesh`)))
  (bind _returnvalue_2 (`SceneComponent.K2_GetComponentLocation` _arrow))
  (`|SpawnActorFromClass` "/Game/VehicleBP/Bullet.Bullet_C" (`KismetMathLibrary.MakeTransform` (+ (`self.K2_GetActorLocation`) (`KismetMathLibrary.GreaterGreater_VectorRotator` (`self.Weapon Offset`) _returnvalue)) _returnvalue) "Undefined" "OverrideRootScale")
  (bind _outhit (`KismetSystemLibrary.LineTraceSingle` :`Start` _returnvalue_2 :`End` (+ _returnvalue_2 (* (`SceneComponent.GetForwardVector` _arrow) 50000.0)) :`TraceChannel` "TraceTypeQuery2" :`bTraceComplex` true :`DrawDebugType` "ForDuration")))

(fn `UserConstructionScript`)