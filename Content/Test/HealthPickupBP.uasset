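; Health pickup actor that restores health to the Sedan vehicle and then destroys itself.
; Every Tick it finds all Sedan actors, takes the first and polls whether that car's mesh overlaps the pickup, rather than using overlap events.
; It adds a fixed amount only when Health is at most 99, with no clamp on the result, so a full-health car leaves it in place.
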(event `self.ReceiveTick`
  (params (DeltaSeconds :type "Float (single-precision)"))
  (bind _outactors (`GameplayStatics.GetAllActorsOfClass` "/Game/VehicleBP/Sedan/Sedan.Sedan_C"))
  (bind _assedan (cast `/Game/VehicleBP/Sedan/Sedan` (`KismetArrayLibrary.Array_Get` _outactors)))
  (if (`PrimitiveComponent.IsOverlappingActor` (`WheeledVehicle.Mesh` _assedan) (`ActorComponent.GetOwner` (`self.Box`)))
    (bind _health (`/Game/VehicleBP/Sedan/Sedan.Health` _assedan))
    (if (<= _health 99.0)
      (set `/Game/VehicleBP/Sedan/Sedan.Health` (+ _health 25.0) _assedan)
      (`self.K2_DestroyActor`))))

(fn `UserConstructionScript`)